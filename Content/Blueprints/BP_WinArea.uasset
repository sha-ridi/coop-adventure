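; BP_WinArea handles the end-of-game win sequence.
; On BeginPlay it binds GameWon to the OnWin dispatcher, which is not fired within these graphs.
; GameWon blocks the first player controller's move and look input, then waits briefly.
; It then shows the WBP_WinScreen widget, reveals the mouse cursor and switches to UI-only input.
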(event Custom|GameWon
  (bind _returnvalue (Game|GetPlayerController 0))
  (bind _returnvalue_2 (Game|GetPlayerController 0))
  (Input|SetIgnoreMoveInput _returnvalue_2 true)
  (Input|SetIgnoreLookInput _returnvalue_2 true)
  (Utilities|FlowControl|Delay 2.0)
  (bind _returnvalue_3 (UserInterface|CreateWidget "/Game/UI/WBP_WinScreen.WBP_WinScreen_C"))
  (UserInterface|Viewport|AddtoViewport _returnvalue_3 0)
  (Variables|/Script/Engine.PlayerController|SetbShowMouseCursor _returnvalue true)
  (Input|SetInputModeUIOnly _returnvalue 0 "DoNotLock" false))

(event EventBeginPlay
  (EventDispatchers|BindEventtoOnWin (delegate Custom|GameWon)))

(fn ConstructionScript)